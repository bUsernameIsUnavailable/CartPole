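; BP_Cartpole is a cart-and-pole rig that moves along X and flags when either part hits something.
; On play it switches the view to its child computer camera and links cart and pole with two constraints.
; Manual axis input offsets the cart, zeroed while GI_Cartpole is in control.
; SaveScreen has GI_Cartpole capture that camera's state as a tensor and write it to a hardcoded Python-folder path.
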(event OnComponentHit(Cart)
  (params (HitComponent :type Primitive%20Component%20Object%20Reference) (OtherActor :type Actor%20Object%20Reference) (OtherComp :type Primitive%20Component%20Object%20Reference) (NormalImpulse :type Vector :default "0, 0, 0") (Hit :type Hit%20Result%20Structure%20%28by%20ref%29))
  (Variables|Default|SetTouchedFlag true))

(event OnComponentHit(Pole)
  (params (HitComponent :type Primitive%20Component%20Object%20Reference) (OtherActor :type Actor%20Object%20Reference) (OtherComp :type Primitive%20Component%20Object%20Reference) (NormalImpulse :type Vector :default "0, 0, 0") (Hit :type Hit%20Result%20Structure%20%28by%20ref%29))
  (Variables|Default|SetTouchedFlag true))

(event EventBeginPlay
  (bind _output_get (Variables|Default|SetCachedCamera (.AsBP%20Computer%20Camera (Utilities|Casting|CastToBP_ComputerCamera (Variables|/Script/Engine.ChildActorComponent|GetChildActor (Variables|Default|GetCamera))))))
  (Game|Player|SetViewTargetwithBlend (Game|GetPlayerController 0) _output_get 0.0 "VTBlend_Linear" 0.0 false)
  (Class|PhysicsConstraintComponent|SetConstrainedComponents (Variables|Default|GetCartConstraint) (Variables|Default|GetCart) "None" (Variables|Default|GetPole) "None")
  (Class|PhysicsConstraintComponent|SetConstrainedComponents (Variables|Default|GetPoleConstraint) (Variables|Default|GetPole) "None" (Variables|Default|GetCart) "None"))

(event Input|ActionEvents|InputActionSaveScreen
  (params (Key :type Key%20Structure :default "None"))
  (bind _returnvalue (Game|GetGameInstance))
  (bind _asgi_cartpole (Utilities|Casting|CastToGI_Cartpole _returnvalue))
  (:Pressed
    (bind _statetensor (Default|ObtainCurrentState _asgi_cartpole (Variables|Default|GetCachedCamera)))
    (Default|TensorasBytes _asgi_cartpole _statetensor "B:\\Cartpole\\Python\\Observation")))

(event Input|AxisEvents|InputAxisMoveLeft
  (params (AxisValue :type Float%20%28single-precision%29))
  (CallFunction|MoveRight (* AxisValue (not (Variables|/Game/GI_Cartpole.GI_Cartpole_C|GetIsInControl (.AsGI%20Cartpole (Utilities|Casting|CastToGI_Cartpole (Game|GetGameInstance))))))))

(event Input|AxisEvents|InputAxisMoveRight
  (params (AxisValue :type Float%20%28single-precision%29))
  (CallFunction|MoveRight (* AxisValue (not (Variables|/Game/GI_Cartpole.GI_Cartpole_C|GetIsInControl (.AsGI%20Cartpole (Utilities|Casting|CastToGI_Cartpole (Game|GetGameInstance))))))))

(fn ConstructionScript)

(fn MoveRight
  (params (Value :type Float%20%28double-precision%29))
  (Transformation|AddWorldOffset (Variables|Default|GetCart) (Math|Vector|MakeVector Value 0.0 0.0) false false))