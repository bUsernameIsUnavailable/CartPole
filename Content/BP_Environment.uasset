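; BP_Environment runs cartpole reinforcement-learning episodes, respawning the BP_Cartpole agent and reloading saved network and optimiser files on each reset.
; While the AI controls, Tick applies the action selected by GI_Cartpole and steps the agent.
; Training stores transitions, runs DQN-style replay updates with epsilon decay every tick, then saves weights and CSV stats at episode end.
; Inference moves with smaller steps; without AI control, the agent's TouchedFlag triggers resets.
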(event Custom|Event%20ResetEnvironment
  (Utilities|IsValid (Variables|Default|GetAgent)
    (:Is%20Valid
      (Actor|DestroyActor (Variables|Default|GetAgent)))
    (:Is%20Not%20Valid
      _))
  (bind _returnvalue (Game|SpawnActorfromClass "/Game/BP_Cartpole.BP_Cartpole_C" (Variables|Default|GetAgentTransform) "AlwaysSpawn" "MultiplyWithRoot" 0 0))
  (Variables|Default|SetAgent _returnvalue)
  (Variables|/Game/GI_Cartpole.GI_Cartpole_C|SetIsDone (Variables|Default|GetGameInstance) false)
  (Variables|/Game/GI_Cartpole.GI_Cartpole_C|SetEpisodeStartTime (Variables|Default|GetGameInstance) (Utilities|Time|GetWorldDeltaSeconds))
  (Variables|/Game/GI_Cartpole.GI_Cartpole_C|SetEpisodeScore (Variables|Default|GetGameInstance) 0)
  (Variables|Default|SetEpisodeStarted true)
  (Default|ObtainCurrentState (Variables|Default|GetGameInstance) (Variables|/Game/BP_Cartpole.BP_Cartpole_C|GetCachedCamera (Variables|Default|GetAgent)))
  (if (Class|BlueprintPathsLibrary|FileExists "B:\\Cartpole\\Content\\Network.pt")
    (Class|AtumSerializable|LoadfromFile (Variables|/Game/GI_Cartpole.GI_Cartpole_C|GetNetwork (Variables|Default|GetGameInstance)) "../../../Content/Network.pt"))
  (if (Class|BlueprintPathsLibrary|FileExists "B:\\Cartpole\\Content\\Optimiser.pt")
    (Class|AtumSerializable|LoadfromFile (Variables|/Game/GI_Cartpole.GI_Cartpole_C|GetAdamOptimiser (Variables|Default|GetGameInstance)) "../../../Content/Optimiser.pt")))

(event EventBeginPlay
  (Variables|Default|SetGameInstance (.AsGI%20Cartpole (Utilities|Casting|CastToGI_Cartpole (Game|GetGameInstance))))
  (CallFunction|EventResetEnvironment))

(event EventTick
  (params (DeltaSeconds :type Float%20%28single-precision%29))
  (bind _gameinstance (Variables|Default|GetGameInstance))
  (bind _gameinstance_2 (Variables|Default|GetGameInstance))
  (bind _gameinstance_3 (Variables|Default|GetGameInstance))
  (bind _gameinstance_4 (Variables|Default|GetGameInstance))
  (if (and (Variables|/Game/GI_Cartpole.GI_Cartpole_C|GetIsInControl (Variables|Default|GetGameInstance)) (Variables|Default|GetEpisodeStarted))
    (if (Variables|/Game/GI_Cartpole.GI_Cartpole_C|GetIsTraining (Variables|Default|GetGameInstance))
      (bind _action (Default|SelectAction (Variables|Default|GetGameInstance)))
      (bind _output_get (Variables|Default|SetActionIndexCache _action))
      (Default|MoveRight (Variables|Default|GetAgent) (Math|Conversions|ToFloat(Integer) (* (- _output_get 1) 15)))
      (bind (_outstate _outreward _outdone) (Default|Step (Variables|Default|GetGameInstance) (Variables|Default|GetAgent)))
      (Default|MemoriseTransitions (Variables|Default|GetGameInstance) _outstate _outreward (Variables|Default|GetActionIndexCache) _outdone)
      (bind _returnvalue (Class|AtumExampleLibrary|Train (Variables|/Game/GI_Cartpole.GI_Cartpole_C|GetNetwork _gameinstance_3) (Variables|/Game/GI_Cartpole.GI_Cartpole_C|GetAdamOptimiser _gameinstance_3) (Math|Integer|Min(Integer) (Variables|/Game/GI_Cartpole.GI_Cartpole_C|GetMemoryIndex _gameinstance_3) (Variables|/Game/GI_Cartpole.GI_Cartpole_C|GetMemorySize _gameinstance_3)) 32 (Variables|/Game/GI_Cartpole.GI_Cartpole_C|GetEpsilon _gameinstance_3) 0.0 0.999 0.99 (Variables|/Game/GI_Cartpole.GI_Cartpole_C|GetStateMemory _gameinstance_3) (Variables|/Game/GI_Cartpole.GI_Cartpole_C|GetNewStateMemory _gameinstance_3) (Variables|/Game/GI_Cartpole.GI_Cartpole_C|GetRewardMemory _gameinstance_3) (Variables|/Game/GI_Cartpole.GI_Cartpole_C|GetActionMemory _gameinstance_3) (Variables|/Game/GI_Cartpole.GI_Cartpole_C|GetTerminalMemory _gameinstance_3) (Variables|/Game/GI_Cartpole.GI_Cartpole_C|GetLoss _gameinstance_3) (Variables|/Game/GI_Cartpole.GI_Cartpole_C|GetDevice _gameinstance_3)))
      (Variables|/Game/GI_Cartpole.GI_Cartpole_C|SetEpsilon _gameinstance_4 _returnvalue)
      (if (Variables|/Game/GI_Cartpole.GI_Cartpole_C|GetIsDone _gameinstance_4)
        (Class|AtumSerializable|SavetoFile (Variables|/Game/GI_Cartpole.GI_Cartpole_C|GetNetwork _gameinstance_2) "../../../Content/Network.pt")
        (Class|AtumSerializable|SavetoFile (Variables|/Game/GI_Cartpole.GI_Cartpole_C|GetAdamOptimiser _gameinstance_2) "../../../Content/Optimiser.pt")
        (Class|AtumExampleLibrary|SaveEpisodeData (Variables|/Game/GI_Cartpole.GI_Cartpole_C|GetEpisodeCount _gameinstance) (Variables|/Game/GI_Cartpole.GI_Cartpole_C|GetEpisodeScore _gameinstance) (Variables|/Game/GI_Cartpole.GI_Cartpole_C|GetEpsilon _gameinstance) (Variables|/Game/GI_Cartpole.GI_Cartpole_C|GetLoss _gameinstance) "B:\\Cartpole\\Content\\EpisodeData.csv")
        (Math|Integer|IncrementInt (Variables|/Game/GI_Cartpole.GI_Cartpole_C|GetEpisodeCount (Variables|Default|GetGameInstance))
          (:%20%20
            (CallFunction|EventResetEnvironment))))
      (else
        (bind _action_2 (Default|SelectAction (Variables|Default|GetGameInstance)))
        (Default|MoveRight (Variables|Default|GetAgent) (Math|Conversions|ToFloat(Integer) (* (- _action_2 1) 6)))
        (bind _outdone_2 (Default|Step (Variables|Default|GetGameInstance) (Variables|Default|GetAgent)))
        (if _outdone_2
          (CallFunction|EventResetEnvironment))))
    (elif (Variables|/Game/BP_Cartpole.BP_Cartpole_C|GetTouchedFlag (Variables|Default|GetAgent))
      (CallFunction|EventResetEnvironment))))

(fn ConstructionScript)